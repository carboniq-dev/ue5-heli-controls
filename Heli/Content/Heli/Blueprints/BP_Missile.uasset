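; BP_Missile is a missile actor, apparently for the helicopter, that explodes on contact.
; On BeginPlay it binds to its OnBurn dispatcher, which activates the NSFlame effect when fired.
; A Collision overlap with anything not exactly of class BP_Heli or BP_Missile spawns the NS_Explosion Niagara system and destroys the missile.
; The graph applies no damage and contains no movement logic.
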(event `self.ReceiveBeginPlay`
  ;[1 1 1] Bind Fire Delegate
  (add `self.OnBurn` (delegate `OnBurn_Event_0`)))

(event `OnBurn_Event_0`
  ;[1 1 1] Bind Fire Delegate
  (`ActorComponent.Activate` (`self.NS_Flame`) true))

(event `self.Collision.OnComponentBeginOverlap`
  (params (OverlappedComponent :type "PrimitiveComponent Object Reference") (OtherActor :type "Actor Object Reference") (OtherComp :type "PrimitiveComponent Object Reference") (OtherBodyIndex :type Integer) (bFromSweep :type Boolean) (SweepResult :type "HitResult Structure (by ref)"))
  (bind _returnvalue (`GameplayStatics.GetObjectClass` OtherActor))
  (if (not (or (== _returnvalue "/Game/Heli/Blueprints/BP_Heli.BP_Heli_C") (== _returnvalue "BP_Missile_C")))
    (`NiagaraFunctionLibrary.SpawnSystemAtLocation` "/Game/Heli/FX/NS_Explosion.NS_Explosion" (`self.K2_GetActorLocation`))
    (`self.K2_DestroyActor`)))

(fn `UserConstructionScript`)